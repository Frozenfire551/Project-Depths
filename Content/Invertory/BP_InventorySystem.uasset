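; Inventory system that tracks item quantities and capacities in a Content array of predefined slots, using DT_ItemList for item data.
; AddItem increases a matching slot by item type, clamping Ammo at capacity and never creating slots.
; Capacity upgrades rely on slot order: Health raises the first slot's capacity, Money sets the preceding slot's from DT_ItemUPgrades via GetnewCap.
; FindKey consumes one key and reports success; RemoveItem is an empty stub.
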(event EventBeginPlay)

(fn AddItem
  (params (ItemInfo :type F%20Item%20on%20Ground%20Structure))
  (bind (_itemid _derstion _quity _displayname _itemtype) (Utilities|Struct|BreakFItemOnGround ItemInfo))
  (bind _content (Variables|Default|GetContent))
  (bind _output (Utilities|Array|Get(acopy) _content))
  (bind (_itemid_2 _quantity _capacity) (Utilities|Struct|BreakFInventoryStruct _output))
  (bind (_array_element _array_index) (Utilities|Array|ForEachLoopwithBreak (Variables|Default|GetContent) :!label _label)
    (:LoopBody
      (if (== (.ItemID (Utilities|Struct|BreakFInventoryStruct _array_element)) _itemid)
        (bind _returnvalue (Utilities|GetDataTableRow "/Game/Invertory/DT_ItemList.DT_ItemList" _itemid)
          (:then
            (switch Utilities|FlowControl|Switch|SwitchonEItem_Type (.ItemType (Utilities|Struct|BreakFItemStruct _returnvalue))
              (:NewEnumerator0
                _)
              (:NewEnumerator1
                _)
              (:NewEnumerator2
                (if (> (+ (.Quantity (Utilities|Struct|BreakFInventoryStruct _array_element)) _quity) (.Capacity (Utilities|Struct|BreakFInventoryStruct _array_element)))
                  (Utilities|Array|SetArrayElem (Variables|Default|GetContent) _array_index (Utilities|Struct|MakeFInventoryStruct (.ItemID (Utilities|Struct|BreakFInventoryStruct _array_element)) (.Capacity (Utilities|Struct|BreakFInventoryStruct _array_element)) (.Capacity (Utilities|Struct|BreakFInventoryStruct _array_element))))
                  (goto _label Break)
                  (else
                    _)))
              (:NewEnumerator3
                _)
              (:NewEnumerator4
                _)
              (:NewEnumerator5
                _)
              (:NewEnumerator6
                _)
              (:NewEnumerator7
                (switch Utilities|FlowControl|Switch|SwitchonEItem_AmmoType _itemtype
                  (:NewEnumerator0
                    (Utilities|Array|SetArrayElem (Variables|Default|GetContent) _array_index (Utilities|Struct|MakeFInventoryStruct (.ItemID (Utilities|Struct|BreakFInventoryStruct _array_element)) (+ (.Quantity (Utilities|Struct|BreakFInventoryStruct _array_element)) _quity) (.Capacity (Utilities|Struct|BreakFInventoryStruct _array_element))))
                    (Utilities|Array|SetArrayElem (Variables|Default|GetContent) 0 (Utilities|Struct|MakeFInventoryStruct _itemid_2 _quantity (+ _capacity _quity)))
                    (goto _label Break))
                  (:NewEnumerator3
                    (bind _capatiy (CallFunction|GetnewCap (.ItemID (Utilities|Struct|BreakFInventoryStruct (Utilities|Array|Get(acopy) (Variables|Default|GetContent) _array_index))) (+ (.Quantity (Utilities|Struct|BreakFInventoryStruct (Utilities|Array|Get(acopy) (Variables|Default|GetContent) _array_index))) 1)))
                    (Utilities|Array|SetArrayElem (Variables|Default|GetContent) (- _array_index 1) (Utilities|Struct|MakeFInventoryStruct (.ItemID (Utilities|Struct|BreakFInventoryStruct (Utilities|Array|Get(acopy) (Variables|Default|GetContent) (- _array_index 1)))) (.Quantity (Utilities|Struct|BreakFInventoryStruct (Utilities|Array|Get(acopy) (Variables|Default|GetContent) (- _array_index 1)))) _capatiy))))))
            (Utilities|Array|SetArrayElem (Variables|Default|GetContent) _array_index (Utilities|Struct|MakeFInventoryStruct (.ItemID (Utilities|Struct|BreakFInventoryStruct _array_element)) (+ (.Quantity (Utilities|Struct|BreakFInventoryStruct _array_element)) _quity) (.Capacity (Utilities|Struct|BreakFInventoryStruct _array_element))))
            (goto _label Break)))))))

(fn RemoveItem)

(fn GetnewCap
  (params (UpgradeRow :type Name) (Quainty%20 :type Integer))
  (bind _returnvalue (Utilities|GetDataTableRow "/Game/Invertory/DT_ItemUPgrades.DT_ItemUPgrades" UpgradeRow)
    (:then
      (switch int Quainty%20
        (:Default
          (Development|PrintString "can't upgrande anymore"))
        (:0
          (return (.upgrade_0 (Utilities|Struct|BreakFItem_Upgrade _returnvalue))))
        (:1
          (return (.upgrade_1 (Utilities|Struct|BreakFItem_Upgrade _returnvalue))))
        (:2
          (return (.upgrade_2 (Utilities|Struct|BreakFItem_Upgrade _returnvalue))))
        (:3
          (return (.upgrade_3 (Utilities|Struct|BreakFItem_Upgrade _returnvalue))))
        (:4
          (return (.upgrade_4 (Utilities|Struct|BreakFItem_Upgrade _returnvalue))))
        (:5
          (return (.upgrade_5 (Utilities|Struct|BreakFItem_Upgrade _returnvalue))))))))

(fn FindKey
  (params (Key :type Name))
  (bind _returnvalue (Utilities|GetDataTableRow "/Game/Invertory/DT_ItemList.DT_ItemList" Key)
    (:then
      (for (_array_element _array_index) (Variables|Default|GetContent)
        (if (== (.ItemID (Utilities|Struct|BreakFInventoryStruct _array_element)) (.Name (Utilities|Struct|BreakFItemStruct _returnvalue)))
          (if (> (.Quantity (Utilities|Struct|BreakFInventoryStruct _array_element)) 0)
            (Utilities|Array|SetArrayElem (Variables|Default|GetContent) _array_index (Utilities|Struct|MakeFInventoryStruct (.ItemID (Utilities|Struct|BreakFInventoryStruct _array_element)) (- (.Quantity (Utilities|Struct|BreakFInventoryStruct _array_element)) 1) (.Capacity (Utilities|Struct|BreakFInventoryStruct _array_element))))
            (return true))))
      (return false))))