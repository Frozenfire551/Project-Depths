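; Interactable door Blueprint that automatically walks the player through the doorway from whichever side they approach.
; Interact converts the player's location into door-local space and uses the sign of X to choose the direction.
; With input disabled, SimpleMoveToLocation sends the player to a scaled offset on the near side, then after a fixed delay to the far side.
; Input returns as soon as the second move is issued, followed by an enter/exit debug print.
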(event EventBeginPlay
  (|CallParentFunction) ; This node is disabled and will not be called.\nDrag off pins to build functionality.
)

(event Collision|EventActorBeginOverlap
  (params (OtherActor :type Actor%20Object%20Reference))
  (|CallParentFunction OtherActor) ; This node is disabled and will not be called.\nDrag off pins to build functionality.
)

(event EventTick
  (params (DeltaSeconds :type Float%20%28single-precision%29))
  (|CallParentFunction DeltaSeconds) ; This node is disabled and will not be called.\nDrag off pins to build functionality.
)

(event EventInteract
  (params (PlayerCharacter :type Actor%20Object%20Reference))
  (bind _returnvalue (Game|GetPlayerController 0))
  (bind _returnvalue_2 (Transformation|GetActorRotation))
  (bind _returnvalue_3 (Game|GetPlayerController 0))
  (bind _defaultsceneroot (Variables|Default|GetDefaultSceneRoot))
  (bind _scale (Variables|Default|Getscale))
  (bind _returnvalue_4 (Transformation|GetWorldLocation _defaultsceneroot))
  (bind _returnvalue_5 (Math|Vector|GetForwardVector _returnvalue_2))
  (bind _returnvalue_6 (* _returnvalue_5 _scale))
  (bind _returnvalue_7 (- _returnvalue_4 _returnvalue_6))
  (bind _returnvalue_8 (+ _returnvalue_4 _returnvalue_6))
  (if (<= (.X (Math|Vector|BreakVector (Math|Transform|InverseTransformLocation (Transformation|GetActorTransform) (Transformation|GetActorLocation PlayerCharacter)))) 0.0)
    (Input|DisableInput PlayerCharacter _returnvalue_3)
    (AI|Navigation|SimpleMovetoLocation _returnvalue_3 _returnvalue_7)
    (Utilities|FlowControl|Delay 2.0)
    (AI|Navigation|SimpleMovetoLocation _returnvalue_3 _returnvalue_8)
    (Input|EnableInput PlayerCharacter _returnvalue_3)
    (Development|PrintString "enter")
    (else
      (Input|DisableInput PlayerCharacter _returnvalue)
      (AI|Navigation|SimpleMovetoLocation _returnvalue _returnvalue_8)
      (Utilities|FlowControl|Delay 2.0)
      (AI|Navigation|SimpleMovetoLocation _returnvalue _returnvalue_7)
      (Input|EnableInput PlayerCharacter _returnvalue)
      (Development|PrintString "exit"))))

(fn ConstructionScript
  (|CallParentFunction))