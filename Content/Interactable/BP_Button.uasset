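; BP_Button is an interactable button whose Interact event currently only prints debug messages.
; It checks the OnlyOnce and ButtonBeenPushed flags to tell a used single-press button from one that can still be pushed.
; The graph never sets ButtonBeenPushed or triggers any other action, and the default events and construction script add no logic.
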(event EventBeginPlay
  (|CallParentFunction) ; This node is disabled and will not be called.\nDrag off pins to build functionality.
)

(event Collision|EventActorBeginOverlap
  (params (OtherActor :type Actor%20Object%20Reference))
  (|CallParentFunction OtherActor) ; This node is disabled and will not be called.\nDrag off pins to build functionality.
)

(event EventTick
  (params (DeltaSeconds :type Float%20%28single-precision%29))
  (|CallParentFunction DeltaSeconds) ; This node is disabled and will not be called.\nDrag off pins to build functionality.
)

(event EventInteract
  (params (PlayerCharacter :type Actor%20Object%20Reference))
  (if (and (== (Variables|Default|GetOnlyOnce) (Variables|Default|GetButtonBeenPushed)) (Variables|Default|GetOnlyOnce))
    (Development|PrintString "OnlyOnceand bushed")
    (else
      (Development|PrintString "can still be pusherd"))))

(fn ConstructionScript
  (|CallParentFunction))